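; Rail track Blueprint that lays a rail mesh along an editable spline to build bendable tracks.
; The construction script divides the spline length by the mesh's X bounding-box extent and adds a spline mesh component per step, attached to the spline.
; Each segment takes its start and end positions and tangents from local-space distances along the spline.
; The event graph has no runtime logic.
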(fn `UserConstructionScript`
  (bind _spline (`self.Spline`))
  (bind _x (.x (`.Max` (break `Box` (`StaticMesh.GetBoundingBox` (`self.Rails_mesh`))))))
  (set `self.Rails_mesh_length` _x)
  (for _index (range (+ (`.ReturnValue` (`KismetMathLibrary.FMod` (`SplineComponent.GetSplineLength` (`self.Spline`)) _x)) 1))
    (bind _returnvalue (`AddComponent|NODE_AddSplineMeshComponent-0` :`bManualAttachment` true))
    (`StaticMeshComponent.SetStaticMesh` _returnvalue (`self.Rails_mesh`))
    (`SceneComponent.K2_AttachToComponent` _returnvalue _spline "None" "KeepRelative" "KeepRelative" "KeepRelative" true)
    (bind _returnvalue_2 (* _index _x))
    (bind _returnvalue_3 (* (+ _index 1) _x))
    (`SplineMeshComponent.SetStartAndEnd` _returnvalue (`SplineComponent.GetLocationAtDistanceAlongSpline` _spline _returnvalue_2 "Local") (`SplineComponent.GetTangentAtDistanceAlongSpline` _spline _returnvalue_2 "Local") (`SplineComponent.GetLocationAtDistanceAlongSpline` _spline _returnvalue_3 "Local") (`SplineComponent.GetTangentAtDistanceAlongSpline` _spline _returnvalue_3 "Local") true)))